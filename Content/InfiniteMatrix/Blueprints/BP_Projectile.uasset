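; BP_Projectile is a projectile actor that flies along the world X axis and expires after a short lifespan.
; Tick applies a swept world offset scaled by MoveSpeed until HasCollided is set.
; The Collided function runs its effect once: it activates the particle system, hides the cube, disables box and cube collision, and resets the lifespan so the effect shows before destruction.
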(event `self.ReceiveBeginPlay`
  (`self.SetLifeSpan` 5.0))

(event `self.ReceiveTick`
  (params (DeltaSeconds :type "Float (single-precision)"))
  (if (not (`self.HasCollided`))
    (`self.K2_AddActorWorldOffset` (`KismetMathLibrary.MakeVector` (* (`self.MoveSpeed`) DeltaSeconds)) true)))

(fn `Collided`
  (if (not (`self.HasCollided`))
    (set `self.HasCollided` true)
    (`ActorComponent.Activate` (`self.ParticleSystem`) false)
    (`self.SetLifeSpan` 2.0)
    (`SceneComponent.SetVisibility` (`self.Cube`) false false)
    (`PrimitiveComponent.SetCollisionEnabled` (`self.Box`) "NoCollision")
    (`PrimitiveComponent.SetCollisionEnabled` (`self.Cube`) "NoCollision")))

(fn `UserConstructionScript`)