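; Spawner actor that builds a chain of BP_Tunnel segments, starting at the player pawn's location.
; On BeginPlay it destroys existing tunnels, then spawns a few, placing each new one at the previous tunnel's Spawnpoint.
; Each tunnel receives a reference to the spawner, runs its randomize function and gets a random rotation speed and direction.
; The spawner tracks the newest tunnel so SpawnTunnelAtSpawnPoint can extend the chain.
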(event `self.ReceiveBeginPlay`
  (`self.Spawn Inital Tunnels`))

(fn `Spawn Inital Tunnels`
  (`|ExecutionSequence`
    (:`then_0`
      (bind _outactors (`GameplayStatics.GetAllActorsOfClass` "/Game/InfiniteMatrix/Blueprints/BP_Tunnel.BP_Tunnel_C"))
      (for _array_element _outactors
        (`self.K2_DestroyActor` _array_element)))
    (:`then_1`
      (for _ (range 3)
        (`/Engine/EditorBlueprintResources/StandardMacros.IsValid` (`self.Newest Tunnel`)
          (:`Is Valid`
            (`self.Spawn Tunnel at Spawn Point`))
          (:`Is Not Valid`
            (`self.SpawnTunnel` (`self.K2_GetActorLocation` (`GameplayStatics.GetPlayerPawn` 0)))))))))

(fn `Spawn Tunnel at Spawn Point`
  (`self.SpawnTunnel` (`SceneComponent.K2_GetComponentLocation` (`/Game/InfiniteMatrix/Blueprints/BP_Tunnel.Spawnpoint` (`self.Newest Tunnel`)))))

(fn `SpawnTunnel`
  (params (SpawnLocation :type "Vector Structure"))
  (bind _returnvalue (`|SpawnActorFromClass` "/Game/InfiniteMatrix/Blueprints/BP_Tunnel.BP_Tunnel_C" (`KismetMathLibrary.MakeTransform` SpawnLocation) "Undefined" "OverrideRootScale" null null))
  (bind _output_get (set `self.Newest Tunnel` _returnvalue))
  (set `/Game/InfiniteMatrix/Blueprints/BP_Tunnel.TunnelSpawner` self _output_get)
  (`/Game/InfiniteMatrix/Blueprints/BP_Tunnel.Randomize Function` _output_get)
  (set `/Game/InfiniteMatrix/Blueprints/BP_Tunnel.RotateSpeed` (* (`KismetMathLibrary.RandomFloatInRange` 20.0 40.0) (`KismetMathLibrary.Conv_IntToDouble` (select `int` (`KismetMathLibrary.RandomIntegerInRange` 0 1) :`0` -1 :`1` 1))) _output_get))

(fn `UserConstructionScript`)