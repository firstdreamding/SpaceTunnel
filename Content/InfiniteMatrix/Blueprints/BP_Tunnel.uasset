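; BP_Tunnel is a tunnel segment with a spinning holed wall, a breakable cube and random health pack and enemy spawns on BeginPlay.
; Player overlap with TriggerZone has TunnelSpawner add another segment, then awards score and destroys this one if unhit.
; The first wall or cube hit damages the player, possibly showing restart; projectiles collide with both, destroying the cube.
; RandomizeFunction, not called here, picks a hole mesh and roll.
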(event `self.ReceiveBeginPlay`
  (bind (_returnvalue_x _returnvalue_y _returnvalue_z) (`KismetMathLibrary.BreakVector` (`SceneComponent.K2_GetComponentLocation` (`self.EnemySpawn`))))
  (bind (_returnvalue_x_2 _returnvalue_y_2 _returnvalue_z_2) (`KismetMathLibrary.BreakVector` (`SceneComponent.K2_GetComponentLocation` (`self.HeathPackSpawn`))))
  (if (== (`KismetMathLibrary.RandomIntegerInRange` 0 9) 0)
    (`|SpawnActorFromClass` "/Game/InfiniteMatrix/Blueprints/BP_HeathPack.BP_HeathPack_C" (`KismetMathLibrary.MakeTransform` (`KismetMathLibrary.MakeVector` _returnvalue_x_2 (+ _returnvalue_y_2 (`KismetMathLibrary.RandomFloatInRange` -200.0 200.0)) (+ _returnvalue_z_2 (`KismetMathLibrary.RandomFloatInRange` -200.0 200.0)))) "Undefined" "OverrideRootScale" null null))
  (if (== (`KismetMathLibrary.RandomIntegerInRange` 0 2) 0)
    (`|SpawnActorFromClass` "/Game/InfiniteMatrix/Blueprints/BP_Enemy.BP_Enemy_C" (`KismetMathLibrary.MakeTransform` (`KismetMathLibrary.MakeVector` _returnvalue_x (+ _returnvalue_y (`KismetMathLibrary.RandomFloatInRange` -100.0 100.0)) (+ _returnvalue_z (`KismetMathLibrary.RandomFloatInRange` -100.0 100.0)))) "Undefined" "OverrideRootScale" null null)))

(event `self.ReceiveTick`
  (params (DeltaSeconds :type "Float (single-precision)"))
  (`SceneComponent.K2_AddLocalRotation` (`self.WallMesh`) (`KismetMathLibrary.MakeRotator` (* DeltaSeconds (`self.RotateSpeed`))) false false))

(event `self.TriggerZone.OnComponentBeginOverlap`
  (params (OverlappedComponent :type "PrimitiveComponent Object Reference") (OtherActor :type "Actor Object Reference") (OtherComp :type "PrimitiveComponent Object Reference") (OtherBodyIndex :type Integer) (bFromSweep :type Boolean) (SweepResult :type "HitResult Structure (by ref)"))
  (cast `/Game/InfiniteMatrix/Blueprints/BP_Player` OtherActor)
  (`/Game/InfiniteMatrix/Blueprints/BP_TunnelSpawner.Spawn Tunnel at Spawn Point` (`self.TunnelSpawner`))
  (if (not (`self.HasHit`))
    (bind _asbp_player (cast `/Game/InfiniteMatrix/Blueprints/BP_Player` (`GameplayStatics.GetPlayerPawn` 0)))
    (set `/Game/InfiniteMatrix/Blueprints/BP_Player.Score` (+ (`self.ScoreWorth`) (`/Game/InfiniteMatrix/Blueprints/BP_Player.Score` _asbp_player)) _asbp_player)
    (`self.K2_DestroyActor`)))

(event `self.WallMesh.OnComponentHit`
  (params (HitComponent :type "PrimitiveComponent Object Reference") (OtherActor :type "Actor Object Reference") (OtherComp :type "PrimitiveComponent Object Reference") (NormalImpulse :type "Vector Structure") (Hit :type "HitResult Structure (by ref)"))
  (bind _asbp_player (cast `/Game/InfiniteMatrix/Blueprints/BP_Player` OtherActor))
  (if (not (`self.HasHit`))
    (set `self.HasHit` true)
    (bind _output_get (set `/Game/InfiniteMatrix/Blueprints/BP_Player.CurrentHP` (- (`/Game/InfiniteMatrix/Blueprints/BP_Player.CurrentHP` _asbp_player) (`self.WallDamage`)) _asbp_player))
    (if (<= _output_get 0)
      (set `/Game/InfiniteMatrix/Blueprints/BP_Player.IsDead` true _asbp_player)
      (`/Game/InfiniteMatrix/Blueprints/BP_Player.DisplayRestart` _asbp_player)
      (else
        (`PrimitiveComponent.SetCollisionEnabled` (`self.WallMesh`) "NoCollision")))))

(event `self.WallMesh.OnComponentBeginOverlap`
  (params (OverlappedComponent :type "PrimitiveComponent Object Reference") (OtherActor :type "Actor Object Reference") (OtherComp :type "PrimitiveComponent Object Reference") (OtherBodyIndex :type Integer) (bFromSweep :type Boolean) (SweepResult :type "HitResult Structure (by ref)"))
  (bind _asprojectile (cast `/Game/InfiniteMatrix/Blueprints/BP_Projectile` OtherActor))
  (`/Game/InfiniteMatrix/Blueprints/BP_Projectile.Collided` _asprojectile))

(event `self.Cube.OnComponentHit`
  (params (HitComponent :type "PrimitiveComponent Object Reference") (OtherActor :type "Actor Object Reference") (OtherComp :type "PrimitiveComponent Object Reference") (NormalImpulse :type "Vector Structure") (Hit :type "HitResult Structure (by ref)"))
  (bind _asbp_player (cast `/Game/InfiniteMatrix/Blueprints/BP_Player` OtherActor))
  (`ActorComponent.K2_DestroyComponent` (`self.Cube`))
  (if (not (`self.HasHit`))
    (set `self.HasHit` true)
    (bind _output_get (set `/Game/InfiniteMatrix/Blueprints/BP_Player.CurrentHP` (- (`/Game/InfiniteMatrix/Blueprints/BP_Player.CurrentHP` _asbp_player) (`self.WallDamage`)) _asbp_player))
    (if (<= _output_get 0)
      (set `/Game/InfiniteMatrix/Blueprints/BP_Player.IsDead` true _asbp_player)
      (`/Game/InfiniteMatrix/Blueprints/BP_Player.DisplayRestart` _asbp_player))))

(event `self.Cube.OnComponentBeginOverlap`
  (params (OverlappedComponent :type "PrimitiveComponent Object Reference") (OtherActor :type "Actor Object Reference") (OtherComp :type "PrimitiveComponent Object Reference") (OtherBodyIndex :type Integer) (bFromSweep :type Boolean) (SweepResult :type "HitResult Structure (by ref)"))
  (bind _asprojectile (cast `/Game/InfiniteMatrix/Blueprints/BP_Projectile` OtherActor))
  (`/Game/InfiniteMatrix/Blueprints/BP_Projectile.Collided` _asprojectile)
  (`ActorComponent.K2_DestroyComponent` (`self.Cube`)))

(fn `Randomize Function`
  (`StaticMeshComponent.SetStaticMesh` (`self.WallMesh`) (select `int` (`KismetMathLibrary.RandomIntegerInRange` 0 3) :`0` "/Game/InfiniteMatrix/Meshes/SM_Hole_01.SM_Hole_01" :`1` "/Game/InfiniteMatrix/Meshes/SM_Hole_02.SM_Hole_02" :`2` "/Game/InfiniteMatrix/Meshes/SM_Hole_03.SM_Hole_03" :`3` "/Game/InfiniteMatrix/Meshes/SM_Hole_04.SM_Hole_04" :!type "StaticMesh Object Reference"))
  (`SceneComponent.K2_AddLocalRotation` (`self.WallMesh`) (`KismetMathLibrary.MakeRotator` (`KismetMathLibrary.RandomFloatInRange` 0.0 360.0)) false false))

(fn `UserConstructionScript`)