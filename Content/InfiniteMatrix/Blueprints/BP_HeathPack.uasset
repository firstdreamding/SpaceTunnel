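; BP_HeathPack is a spinning health pickup that heals the player on contact and then destroys itself.
; Tick yaws the actor at RotationSpeed, scaled by delta time.
; A component hit from BP_Player on either cube adds HealAmount to CurrentHP, clamped between zero and MaxHP.
; A BP_Projectile overlapping either cube has its Collided function called, leaving the pack intact.
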(event `self.ReceiveTick`
  (params (DeltaSeconds :type "Float (single-precision)"))
  (`self.K2_AddActorWorldRotation` (`KismetMathLibrary.MakeRotator` 0.0 0.0 (* DeltaSeconds (`self.RotationSpeed`)))))

(event `self.Cube1.OnComponentHit`
  (params (HitComponent :type "PrimitiveComponent Object Reference") (OtherActor :type "Actor Object Reference") (OtherComp :type "PrimitiveComponent Object Reference") (NormalImpulse :type "Vector Structure") (Hit :type "HitResult Structure (by ref)"))
  (bind _asbp_player (cast `/Game/InfiniteMatrix/Blueprints/BP_Player` OtherActor))
  (set `/Game/InfiniteMatrix/Blueprints/BP_Player.CurrentHP` (`KismetMathLibrary.Clamp` (+ (`/Game/InfiniteMatrix/Blueprints/BP_Player.CurrentHP` _asbp_player) (`self.HealAmount`)) 0 (`/Game/InfiniteMatrix/Blueprints/BP_Player.MaxHP` _asbp_player)) _asbp_player)
  (`self.K2_DestroyActor` :!label _label))

(event `self.Cube.OnComponentHit`
  (params (HitComponent :type "PrimitiveComponent Object Reference") (OtherActor :type "Actor Object Reference") (OtherComp :type "PrimitiveComponent Object Reference") (NormalImpulse :type "Vector Structure") (Hit :type "HitResult Structure (by ref)"))
  (bind _asbp_player (cast `/Game/InfiniteMatrix/Blueprints/BP_Player` OtherActor))
  (set `/Game/InfiniteMatrix/Blueprints/BP_Player.CurrentHP` (`KismetMathLibrary.Clamp` (+ (`/Game/InfiniteMatrix/Blueprints/BP_Player.CurrentHP` _asbp_player) (`self.HealAmount`)) 0 (`/Game/InfiniteMatrix/Blueprints/BP_Player.MaxHP` _asbp_player)) _asbp_player)
  (goto _label))

(event `self.Cube.OnComponentBeginOverlap`
  (params (OverlappedComponent :type "PrimitiveComponent Object Reference") (OtherActor :type "Actor Object Reference") (OtherComp :type "PrimitiveComponent Object Reference") (OtherBodyIndex :type Integer) (bFromSweep :type Boolean) (SweepResult :type "HitResult Structure (by ref)"))
  (bind _asbp_projectile (cast `/Game/InfiniteMatrix/Blueprints/BP_Projectile` OtherActor))
  (`/Game/InfiniteMatrix/Blueprints/BP_Projectile.Collided` _asbp_projectile))

(event `self.Cube1.OnComponentBeginOverlap`
  (params (OverlappedComponent :type "PrimitiveComponent Object Reference") (OtherActor :type "Actor Object Reference") (OtherComp :type "PrimitiveComponent Object Reference") (OtherBodyIndex :type Integer) (bFromSweep :type Boolean) (SweepResult :type "HitResult Structure (by ref)"))
  (bind _asbp_projectile (cast `/Game/InfiniteMatrix/Blueprints/BP_Projectile` OtherActor))
  (`/Game/InfiniteMatrix/Blueprints/BP_Projectile.Collided` _asbp_projectile))

(fn `UserConstructionScript`)